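; Player tank Blueprint that handles component setup, camera aiming and firing.
; On BeginPlay it passes the turret, hull mesh and barrel to setter functions.
; Aim axes yaw the Gimbal and pitch the CameraBoom separately, scaled by frame time and per-axis sensitivity.
; The Fire input calls Fire, whose logic is defined outside these graphs.
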(event `self.ReceiveBeginPlay`
  (`self.SetTurretChildActor` (`self.BP_TankTurret`))
  (`self.SetTankStaticMesh` (`self.TankHull`))
  (`self.SetBarrelReference` (`self.TankBarrel`)))

(event `InputAxis|AimAzimuth`
  (params (AxisValue :type "Float (single-precision)"))
  ;[1 1 1] Player Inputs
  (`SceneComponent.K2_AddLocalRotation` (`self.Gimbal`) (`KismetMathLibrary.MakeRotator` 0.0 0.0 (* AxisValue (`GameplayStatics.GetWorldDeltaSeconds`) (`self.CameraHorizontalSens`))) false false))

(event `InputAxis|AimAltitude`
  (params (AxisValue :type "Float (single-precision)"))
  ;[1 1 1] Player Inputs
  (`SceneComponent.K2_AddLocalRotation` (`self.CameraBoom`) (`KismetMathLibrary.MakeRotator` 0.0 (* AxisValue (`GameplayStatics.GetWorldDeltaSeconds`) (`self.CameraVerticalSens`))) false false))

(event `InputAction|Fire`
  (params (Key :type "Key Structure"))
  ;[1 1 1] Player Inputs
  (:`Pressed`
    (`self.Fire`)))

(fn `UserConstructionScript`)